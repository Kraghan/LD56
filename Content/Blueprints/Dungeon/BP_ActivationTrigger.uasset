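; BP_ActivationTrigger is a dungeon actor with a box trigger volume that expands when the dungeon game mode enters a specific phase.
; On BeginPlay it binds to the phase-changed event of BP_GameModeDungeon.
; For that phase it caches the box's X extent, then the Scaling timeline's curve lerps it to MaxSize, leaving Y and Z unchanged.
; The Blueprint has no overlap logic of its own.
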(event Custom|OnPhaseChanged
  (params (Phase :type E_DungeonPhase%20Enum :default "NewEnumerator0"))
  (bind _box (Variables|Default|GetBox))
  (bind _boxextent (Variables|/Script/Engine.BoxComponent|GetBoxExtent _box))
  (if (Utilities|Enum|Equal(Enum) Phase "NewEnumerator1")
    (Variables|Default|SetBase%20Box%20Extent%20X (.x _boxextent))
    (bind _scalecurve (Timeline|Scaling PlayFromStart)
      (:Update
        (Components|Box|SetBoxExtent _box (Math|Vector|MakeVector (Math|Float|Lerp (Variables|Default|GetBase%20Box%20Extent%20X) (Variables|Default|GetMaxSize) _scalecurve) (.y _boxextent) (.z _boxextent)) true)))))

(event EventBeginPlay
  (bind _asbp_game_mode_dungeon (Utilities|Casting|CastToBP_GameModeDungeon (Game|GetGameMode)))
  (EventDispatchers|BindEventtoOnPhaseChanged _asbp_game_mode_dungeon (EventDispatchers|CreateEvent :!event Custom|OnPhaseChanged)))

(event Collision|EventActorBeginOverlap
  (params (OtherActor :type Actor%20Object%20Reference)))

(event EventTick
  (params (DeltaSeconds :type Float%20%28single-precision%29)))

(fn ConstructionScript)