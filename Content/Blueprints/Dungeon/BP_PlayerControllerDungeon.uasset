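; Player controller for the dungeon that creates its UI and handles placing and removing army units on BP_Grid.
; Game mode phase changes clear the selection and toggle the Preparation input mapping; only the Preparation tick has logic.
; A collision-free preview of the selected unit follows the cursor, snapping to tile centers.
; Placement checks army availability and tile occupancy, replacing different unit types found by sphere overlap, and updates grid occupancy.
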(event Custom|OnGameModePhaseChanged
  (params (Phase :type E_DungeonPhase%20Enum :default "NewEnumerator0"))
  (bind _self self)
  (bind _returnvalue (PlayerController|LocalPlayerSubsystems|GetEnhancedInputLocalPlayerSubsystem _self))
  (CallFunction|SetSelectedUnit)
  (switch Utilities|FlowControl|Switch|SwitchonE_DungeonPhase Phase
    (:NewEnumerator0
      (Input|AddMappingContext _returnvalue (Variables|InputGame|GetInputMappingPreparation) 0 "(bIgnoreAllPressedKeysUntilRelease=True,bForceImmediately=False,bNotifyUserSettings=False)"))
    (:NewEnumerator1
      (Input|RemoveMappingContext _returnvalue (Variables|InputGame|GetInputMappingPreparation) "(bIgnoreAllPressedKeysUntilRelease=True,bForceImmediately=False,bNotifyUserSettings=False)"))))

(event Input|EnhancedActionEvents|EnhancedInputActionIA_PlaceUnit
  (params (ActionValue :type Boolean) (ElapsedSeconds :type Float%20%28double-precision%29) (TriggeredSeconds :type Float%20%28double-precision%29) (InputAction :type Input%20Action%20Object%20Reference :default "/Game/Blueprints/Inputs/IA_PlaceUnit.IA_PlaceUnit"))
  (CallFunction|TrySpawnUnit))

(event Input|EnhancedActionEvents|EnhancedInputActionIA_RemoveUnit
  (params (ActionValue :type Boolean) (ElapsedSeconds :type Float%20%28double-precision%29) (TriggeredSeconds :type Float%20%28double-precision%29) (InputAction :type Input%20Action%20Object%20Reference :default "/Game/Blueprints/Inputs/IA_RemoveUnit.IA_RemoveUnit"))
  (CallFunction|DestroyUnitUnderCursor))

(event EventBeginPlay
  (bind _returnvalue (UserInterface|CreateWidget "/Game/Blueprints/UI/UI_Dungeon.UI_Dungeon_C" self))
  (bind _output_get (Variables|Default|SetUI _returnvalue))
  (UserInterface|Viewport|AddtoViewport _output_get 0)
  (bind _asbp_game_mode_dungeon (Utilities|Casting|CastToBP_GameModeDungeon (Game|GetGameMode)))
  (bind _output_get_2 (Variables|Default|SetGameMode _asbp_game_mode_dungeon))
  (CallFunction|OnGameModePhaseChanged (Variables|/Game/Blueprints/Dungeon/BP_GameModeDungeon.BP_GameModeDungeon_C|GetCurrentDungeonPhase _output_get_2))
  (EventDispatchers|BindEventtoOnPhaseChanged _output_get_2 (EventDispatchers|CreateEvent :!event Custom|OnGameModePhaseChanged))
  (Input|SetInputModeGameandUI self (Variables|Default|GetUI) "DoNotLock" false false)
  (Variables|Default|SetbShowMouseCursor true)
  (bind _returnvalue_2 (Actor|GetActorOfClass "/Game/Blueprints/Dungeon/BP_Grid.BP_Grid_C"))
  (Variables|Default|SetGrid _returnvalue_2)
  (bind _asbp_game_instance (Utilities|Casting|CastToBP_GameInstance (Game|GetGameInstance)))
  (Variables|Default|SetGameInstance _asbp_game_instance))

(event EventTick
  (params (DeltaSeconds :type Float%20%28single-precision%29))
  (switch Utilities|FlowControl|Switch|SwitchonE_DungeonPhase (Variables|/Game/Blueprints/Dungeon/BP_GameModeDungeon.BP_GameModeDungeon_C|GetCurrentDungeonPhase (Variables|Default|GetGameMode))
    (:NewEnumerator0
      (CallFunction|TickPreparationPhase DeltaSeconds))
    (:NewEnumerator1
      (CallFunction|TickBattlePhase DeltaSeconds))
    (:NewEnumerator2
      (CallFunction|TickPostBattlePhase DeltaSeconds))))

(fn ConstructionScript)

(fn SetSelectedUnit
  (params (Unit :type BP%20Unit%20Base%20Class%20Reference))
  (bind _output_get (Variables|Default|SetSelectedUnitToSpawn Unit))
  (bind _unitbasecursor (Variables|Default|GetUnitBaseCursor)
    (:then
      (Actor|DestroyActor _unitbasecursor)
      (Variables|Default|SetUnitBaseCursor 0))
    (:else
      _))
  (if (Utilities|IsValidClass _output_get)
    (bind _returnvalue (Game|SpawnActorfromClass (Variables|Default|GetSelectedUnitToSpawn) (Math|Transform|MakeTransform (CallFunction|GetCursor3DPosition) "0, 0, 0" "1.000000,1.000000,1.000000") "AlwaysSpawn" "MultiplyWithRoot" 0 true false 0))
    (Variables|Default|SetUnitBaseCursor _returnvalue)))

(fn GetCursor3DPosition
  (return (.impactpoint (.HitResult (Game|Player|GetHitResultUnderCursorbyChannel "TraceTypeQuery1" true)))))

(fn TickPreparationPhase
  (params (DeltaTime :type Float%20%28double-precision%29))
  (bind _position (CallFunction|GetCursor3DPosition))
  (bind _grid (Variables|Default|GetGrid))
  (bind (_tilecoordinates _validpos) (Default|LocationtoGridCoordinates _grid _position))
  (bind _unitbasecursor (Variables|Default|GetUnitBaseCursor)
    (:then
      (if _validpos
        (Transformation|SetActorLocation _unitbasecursor (.Position (Default|GridCoordinatestoWorldSpace _grid _tilecoordinates true)) false false)
        (else
          (Transformation|SetActorLocation _position false false))))
    (:else)))

(fn TickBattlePhase
  (params (DeltaTime :type Float%20%28double-precision%29)))

(fn TickPostBattlePhase
  (params (DeltaTime :type Float%20%28double-precision%29)))

(fn TrySpawnUnit
  (bind _outactors (CallFunction|FindUnitUnderCursor))
  (bind _unitbasecursor (Variables|Default|GetUnitBaseCursor))
  (bind _grid (Variables|Default|GetGrid))
  (bind _selectedunittospawn (Variables|Default|GetSelectedUnitToSpawn))
  (bind _returnvalue (Transformation|GetActorLocation _unitbasecursor))
  (bind (_tilecoordinates _validpos) (Default|LocationtoGridCoordinates _grid _returnvalue))
  (if (Utilities|IsValidClass _selectedunittospawn)
    (if (CallFunction|HasAnyAvailableUnitRemaining (Default|GetArmy (Variables|Default|GetGameInstance)) _selectedunittospawn)
      (if _validpos
        (if (Default|IsTileFree _grid _tilecoordinates)
          (Game|SpawnActorfromClass (Variables|Default|GetSelectedUnitToSpawn) (Math|Transform|MakeTransform (+ _returnvalue "0.000000,0.000000,100.000000") "0, 0, 0" "1.000000,1.000000,1.000000") "AdjustIfPossibleButAlwaysSpawn" "MultiplyWithRoot" 0 false true 0 :!label _label)
          (Default|AddOccupiedTile (Variables|Default|GetGrid) _tilecoordinates)
          (else
            (Utilities|IsValid _outactors
              (:Is%20Valid
                (if (not (== (Utilities|GetClass _outactors) (Variables|Default|GetSelectedUnitToSpawn)))
                  (CallFunction|DestroyUnit _outactors)
                  (goto _label)))
              (:Is%20Not%20Valid
                (Development|PrintString "Something weird !"))))))
      (else
        (Default|CallNotEnoughUnitRemaining (Variables|Default|GetSelectedUnitToSpawn))))))

(fn DestroyUnitUnderCursor
  (bind _outactors (CallFunction|FindUnitUnderCursor))
  (Utilities|IsValid _outactors
    (:Is%20Valid
      (CallFunction|DestroyUnit _outactors))))

(fn FindUnitUnderCursor
  (bind _unitbasecursor (Variables|Default|GetUnitBaseCursor))
  (Utilities|IsValid _unitbasecursor
    (:Is%20Valid
      (LocalVariables|SetCheckPos (Transformation|GetActorLocation _unitbasecursor))
      (Utilities|Array|Add (LocalVariables|GetActorToIgnore) _unitbasecursor))
    (:Is%20Not%20Valid
      (LocalVariables|SetCheckPos (CallFunction|GetCursor3DPosition))))
  (bind (_outactors _returnvalue) (Collision|SphereOverlapActors (LocalVariables|GetCheckPos) 5e+01 (Utilities|Array|MakeArray "ObjectTypeQuery3") "/Game/Blueprints/Dungeon/Units/BP_UnitBase.BP_UnitBase_C" (LocalVariables|GetActorToIgnore)))
  (if _returnvalue
    (if (> (Utilities|Array|Length _outactors) 1)
      (Development|PrintString "More than one entity found"))
    (bind _asbp_unit_base (Utilities|Casting|CastToBP_UnitBase (Utilities|Array|Get(acopy) _outactors)))
    (return _asbp_unit_base)
    (else
      (return 0))))

(fn DestroyUnit
  (params (Unit :type BP%20Unit%20Base%20Object%20Reference))
  (bind _grid (Variables|Default|GetGrid))
  (Default|RemoveOccupiedTile _grid (.TileCoordinates (Default|LocationtoGridCoordinates _grid (Transformation|GetActorLocation Unit))))
  (Actor|DestroyActor Unit))