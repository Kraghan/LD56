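; BP_Projectile is a homing projectile fired by a BP_UnitBase instigator in the dungeon game.
; Each Tick it steers toward the Target's last known location by interpolating its direction, moves without sweep, and dies once it passes that point.
; Overlapping an opposing-camp unit applies the firing unit's damage, adjusted for type advantage, then kills it.
; Kill stops movement, adds a Niagara effect and sets a short lifespan.
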(event OnComponentBeginOverlap(Trigger)
  (params (OverlappedComponent :type Primitive%20Component%20Object%20Reference) (OtherActor :type Actor%20Object%20Reference) (OtherComp :type Primitive%20Component%20Object%20Reference) (OtherBodyIndex :type Integer) (bFromSweep :type Boolean) (SweepResult :type Hit%20Result%20Structure%20%28by%20ref%29))
  (bind _unit (Variables|Default|GetUnit))
  (bind _asbp_unit_base (Utilities|Casting|CastToBP_UnitBase OtherActor))
  (if (!= (Variables|/Game/Blueprints/Dungeon/Units/BP_UnitBase.BP_UnitBase_C|GetIsPlayerCamp _unit) (Variables|/Game/Blueprints/Dungeon/Units/BP_UnitBase.BP_UnitBase_C|GetIsPlayerCamp _asbp_unit_base))
    (Default|ApplyDamage _asbp_unit_base (Default|GetDamage _unit (CallFunction|IsUnitStrongAgainst (Variables|/Game/Blueprints/Dungeon/Units/BP_UnitBase.BP_UnitBase_C|GetUnitData _unit) (Variables|/Game/Blueprints/Dungeon/Units/BP_UnitBase.BP_UnitBase_C|GetUnitData _asbp_unit_base))))
    (CallFunction|Kill)))

(event EventBeginPlay
  (bind _asbp_unit_base (Utilities|Casting|CastToBP_UnitBase (Game|GetInstigator)))
  (Variables|Default|SetUnit _asbp_unit_base))

(event Collision|EventActorBeginOverlap
  (params (OtherActor :type Actor%20Object%20Reference)))

(event EventTick
  (params (DeltaSeconds :type Float%20%28single-precision%29))
  (if (not (Variables|Default|Getdead))
    (bind _target (Variables|Default|GetTarget)
      (:then
        (Variables|Default|SetDestination (Transformation|GetActorLocation _target)))
      (:else
        _))
    (CallFunction|UpdateDirection DeltaSeconds)
    (Transformation|SetActorLocation (+ (Transformation|GetActorLocation) (* (Variables|Default|GetDirection) (* (Variables|Default|GetMovementSpeed) DeltaSeconds))) false false)
    (if (< (Math|Vector|DotProduct (Variables|Default|GetDirection) (- (Variables|Default|GetDestination) (Transformation|GetActorLocation))) 0.0)
      (CallFunction|Kill))))

(fn ConstructionScript)

(fn UpdateDirection
  (params (DeltaTime :type Float%20%28double-precision%29))
  (Variables|Default|SetDirection (Math|Interpolation|VInterpTo (Variables|Default|GetDirection) (Math|Vector|Normalize (- (Variables|Default|GetDestination) (Transformation|GetActorLocation))) DeltaTime (Variables|Default|GetAngularVelocity))))

(fn Kill
  (Variables|Default|Setdead true)
  (Actor|SetLifeSpan 0.8)
  (AddComponent|AddNiagaraComponent false))