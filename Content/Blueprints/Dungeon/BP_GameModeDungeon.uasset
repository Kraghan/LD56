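; Game mode for the dungeon that runs an encounter through Preparation, Fight and PostFight phases.
; BeginPlay caches the game instance and sorts the level's end-line actors into player and bot lines, exposed through GetEndline.
; During Fight, Tick polls both armies for defeat, flags a player win if its own Army falls, and advances the phase.
; Each phase change fires an OnPhaseChanged dispatcher.
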(event EventBeginPlay
  (bind _asbp_game_instance (Utilities|Casting|CastToBP_GameInstance (Game|GetGameInstance)))
  (Variables|Default|SetGameInstance _asbp_game_instance)
  (bind _outactors (Actor|GetAllActorsOfClass "/Game/Blueprints/Dungeon/BP_DungeonEndLine.BP_DungeonEndLine_C"))
  (for _array_element _outactors
    (if (Variables|/Game/Blueprints/Dungeon/BP_DungeonEndLine.BP_DungeonEndLine_C|GetIsPlayerEndline _array_element)
      (Variables|Default|SetPlayerEndline _array_element)
      (else
        (Variables|Default|SetBotEndline _array_element)))))

(event EventTick
  (params (DeltaSeconds :type Float%20%28single-precision%29))
  (switch Utilities|FlowControl|Switch|SwitchonE_DungeonPhase (Variables|Default|GetCurrentDungeonPhase)
    (:NewEnumerator1
      (if (CallFunction|IsDefeated (Variables|Default|GetArmy))
        (Variables|Default|SetPlayerHasWon true)
        (CallFunction|ChangetoNextPhase)
        (elif (CallFunction|IsDefeated (Default|GetArmy (Variables|Default|GetGameInstance)))
          (CallFunction|ChangetoNextPhase))))))

(fn ConstructionScript)

(fn ChangetoNextPhase
  (switch Utilities|FlowControl|Switch|SwitchonE_DungeonPhase (Variables|Default|GetCurrentDungeonPhase)
    (:NewEnumerator0
      (Variables|Default|SetCurrentDungeonPhase "NewEnumerator1"))
    (:NewEnumerator1
      (Variables|Default|SetCurrentDungeonPhase "NewEnumerator2")))
  (Default|CallOnPhaseChanged (Variables|Default|GetCurrentDungeonPhase)))

(fn GetEndline
  (params (PlayerLine? :type Boolean))
  (if PlayerLine?
    (return (Variables|Default|GetPlayerEndline))
    (else
      (return (Variables|Default|GetBotEndline)))))