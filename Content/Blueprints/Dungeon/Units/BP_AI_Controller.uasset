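; AI controller for dungeon units that runs their combat behavior tree and shuts it down when they die or the fight ends.
; StartBT launches BT_CreatureCombat and copies the unit's detection and attack radii into the blackboard; nothing in this file calls it.
; Possess caches the BP_UnitBase and binds its death event, while BeginPlay subscribes to game mode phase changes to stop the brain at Post Fight.
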(event Custom|OnPhaseChanged
  (params (Phase :type E_DungeonPhase%20Enum :default "NewEnumerator0"))
  (switch Utilities|FlowControl|Switch|SwitchonE_DungeonPhase Phase
    (:NewEnumerator2
      (AI|Logic|StopLogic (Variables|Default|GetBrainComponent) "End game"))))

(event Custom|OnDeath
  (AI|Logic|StopLogic (Variables|Default|GetBrainComponent) "Dead"))

(event EventBeginPlay
  (bind _asbp_game_mode_dungeon (Utilities|Casting|CastToBP_GameModeDungeon (Game|GetGameMode)))
  (EventDispatchers|BindEventtoOnPhaseChanged _asbp_game_mode_dungeon (EventDispatchers|CreateEvent :!event Custom|OnPhaseChanged)))

(event EventTick
  (params (DeltaSeconds :type Float%20%28single-precision%29)))

(event EventPossess
  (params (PossessedPawn :type Pawn%20Object%20Reference))
  (bind _asbp_unit_base (Utilities|Casting|CastToBP_UnitBase PossessedPawn))
  (bind _output_get (Variables|Default|SetUnit _asbp_unit_base))
  (EventDispatchers|BindEventtoOnDead _output_get (delegate Custom|OnDeath)))

(fn ConstructionScript)

(fn StartBT
  (bind _unit (Variables|Default|GetUnit))
  (bind _unitdata (Variables|/Game/Blueprints/Dungeon/Units/BP_UnitBase.BP_UnitBase_C|GetUnitData _unit))
  (AI|RunBehaviorTree "/Game/Blueprints/Dungeon/AI/BT_CreatureCombat.BT_CreatureCombat")
  (AI|Components|Blackboard|SetValueasFloat (AI|GetBlackboard 0) (Variables|Default|GetBBKey_DetectionRadius) (.detectionradius _unitdata))
  (AI|Components|Blackboard|SetValueasFloat (AI|GetBlackboard 0) (Variables|Default|GetBBKey_CombatRadius) (.attackradius _unitdata)))