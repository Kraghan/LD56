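; Clickable hut building in the village that opens an upgrade-related building panel.
; On click, it casts to the village player controller and tells its UiVillage widget to show the Flying or Armored building view, chosen by the Modifier variable.
; Cursor hover toggles custom depth rendering on the hut component.
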(event OnClicked(HUT_A)
  (params (TouchedComponent :type Primitive%20Component%20Object%20Reference) (ButtonPressed :type Key%20Structure :default "None"))
  (bind _asbp_player_controller_village (Utilities|Casting|CastToBp_PlayerController_Village (Game|GetPlayerController 0)))
  (switch Utilities|FlowControl|Switch|SwitchonE_UnitModifier (Variables|Default|GetModifier)
    (:NewEnumerator2
      (Default|ShowBuildingFlying (Variables|/Game/Blueprints/Village/Bp_PlayerController_Village.Bp_PlayerController_Village_C|GetUiVillage _asbp_player_controller_village)))
    (:NewEnumerator3
      (Default|ShowBuildingArmored (Variables|/Game/Blueprints/Village/Bp_PlayerController_Village.Bp_PlayerController_Village_C|GetUiVillage _asbp_player_controller_village)))))

(event OnBeginCursorOver(HUT_A)
  (params (TouchedComponent :type Primitive%20Component%20Object%20Reference))
  (Rendering|SetRenderCustomDepth (Variables|Default|GetHUT_A) true))

(event OnEndCursorOver(HUT_A)
  (params (TouchedComponent :type Primitive%20Component%20Object%20Reference))
  (Rendering|SetRenderCustomDepth (Variables|Default|GetHUT_A) false))

(event EventBeginPlay)

(event Collision|EventActorBeginOverlap
  (params (OtherActor :type Actor%20Object%20Reference)))

(event EventTick
  (params (DeltaSeconds :type Float%20%28single-precision%29)))

(fn ConstructionScript)