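; Actor component for Village blueprints that adds mouse hover highlighting and click toggling to its owning actor.
; On BeginPlay it binds the owner's click event, then caches the owner's static mesh and binds cursor-over events if one exists.
; Hover toggles the mesh's custom depth rendering.
; Each click flips IsClicked and swaps the first material between green and red debug instances.
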(event Custom|OnMouseClicked
  (params (TouchedActor :type Actor%20Object%20Reference) (ButtonPressed :type Key%20Structure :default "None"))
  (bind _staticmeshref (Variables|Default|GetStaticMeshRef))
  (bind _output_get (Variables|Composants|SetIsClicked (not (Variables|Composants|GetIsClicked))))
  (Utilities|IsValid (Variables|Default|GetStaticMeshRef)
    (:Is%20Valid
      (if _output_get
        (Rendering|Material|SetMaterial _staticmeshref 0 "/Game/_MATERIALS/Materials_DEBUG/MI_Debug_Green.MI_Debug_Green")
        (else
          (Rendering|Material|SetMaterial _staticmeshref 0 "/Game/_MATERIALS/Materials_DEBUG/MI_Debug_Red.MI_Debug_Red"))))))

(event Custom|OnMousHover
  (params (TouchedActor :type Actor%20Object%20Reference))
  (Rendering|SetRenderCustomDepth (Variables|Default|GetStaticMeshRef) true))

(event Custom|OnMouseHoverEnd
  (params (TouchedActor :type Actor%20Object%20Reference))
  (Rendering|SetRenderCustomDepth (Variables|Default|GetStaticMeshRef) false))

(event EventBeginPlay
  (bind _returnvalue (Components|GetOwner))
  (bind _returnvalue_2 (Actor|GetComponentbyClass _returnvalue "/Script/Engine.StaticMeshComponent"))
  (EventDispatchers|BindEventtoOnClicked _returnvalue (delegate Custom|OnMouseClicked))
  (Utilities|IsValid _returnvalue_2
    (:Is%20Valid
      (Variables|Default|SetStaticMeshRef _returnvalue_2)
      (EventDispatchers|BindEventtoOnBeginCursorOver _returnvalue (delegate Custom|OnMousHover))
      (EventDispatchers|BindEventtoOnEndCursorOver _returnvalue (delegate Custom|OnMouseHoverEnd)))))