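; Village building actor that represents a unit class and opens its building UI when clicked.
; The construction script reads the unit type from UnitBase class defaults to set the displayed weapon mesh, rescaling it for spears and clearing it for fireball units.
; Hovering the hut toggles custom depth rendering for highlighting.
; Clicking passes UnitBase to the village UI through the village player controller.
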(event OnClicked(HUT_A)
  (params (TouchedComponent :type Primitive%20Component%20Object%20Reference) (ButtonPressed :type Key%20Structure))
  (bind _asbp_player_controller_village (Utilities|Casting|CastToBp_PlayerController_Village (Game|GetPlayerController 0)))
  (Default|ShowBuildingBase (Variables|/Game/Blueprints/Village/Bp_PlayerController_Village.Bp_PlayerController_Village_C|GetUiVillage _asbp_player_controller_village) (Variables|Default|GetUnitBase)))

(event OnBeginCursorOver(HUT_A)
  (params (TouchedComponent :type Primitive%20Component%20Object%20Reference))
  (Rendering|SetRenderCustomDepth (Variables|Default|GetHUT_A) true))

(event OnEndCursorOver(HUT_A)
  (params (TouchedComponent :type Primitive%20Component%20Object%20Reference))
  (Rendering|SetRenderCustomDepth (Variables|Default|GetHUT_A) false))

(event EventBeginPlay)

(event Collision|EventActorBeginOverlap
  (params (OtherActor :type Actor%20Object%20Reference)))

(event EventTick
  (params (DeltaSeconds :type Float%20%28single-precision%29)))

(fn ConstructionScript
  (bind _weapon_sword (Variables|Default|GetWEAPON_SWORD))
  (switch Utilities|FlowControl|Switch|SwitchonE_UnitType (.unittype (.UnitData (Utilities|GetClassDefaults (Variables|Default|GetUnitBase))))
    (:NewEnumerator0
      (Components|StaticMesh|SetStaticMesh _weapon_sword "/Game/_MESH/WEAPONS/WEAPON_AXE.WEAPON_AXE"))
    (:NewEnumerator2
      (Components|StaticMesh|SetStaticMesh _weapon_sword "/Game/_MESH/WEAPONS/WEAPON_SWORD.WEAPON_SWORD"))
    (:NewEnumerator3
      (Components|StaticMesh|SetStaticMesh _weapon_sword "/Game/_MESH/WEAPONS/WEAPON_TRIDENT.WEAPON_TRIDENT")
      (Transformation|SetRelativeScale3D _weapon_sword "1.750000,1.750000,1.000000"))
    (:NewEnumerator1
      (Components|StaticMesh|SetStaticMesh _weapon_sword 0))))