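; Blueprint function library for armies: manages unit counts and rates unit-versus-unit matchups.
; Each army holds owned and engaged unit lists; available count is their difference, and defeat means every owned quantity is zero.
; Matchups sum a weapon triangle (Fire Ball counters Flying) and a modifier advantage for Flying into a clamped five-tier rating from Inoffensive to Lethal.
; IsBetterEncounter ranks two ratings, with Lethal always counting as better, even against Lethal.
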(fn AddUnit
  (params (Army :type ST%20Army%20Structure%20%28by%20ref%29) (UnitBase :type BP%20Unit%20Base%20Class%20Reference) (Quantity :type Integer))
  (for (_array_element _array_index) (.army Army)
    (if (== (.unit _array_element) UnitBase)
      (|SetBy-RefVar (.quantity (Utilities|Array|Get(acopy) (.army Army) _array_index)) (+ (.quantity _array_element) Quantity))
      (return)))
  (Utilities|Array|Add (.army Army) (Utilities|Struct|MakeST_ArmyData UnitBase Quantity)))

(fn RemoveUnit
  (params (Army :type ST%20Army%20Structure%20%28by%20ref%29) (Unit :type BP%20Unit%20Base%20Class%20Reference) (Quantity :type Integer))
  (for (_array_element _array_index) (.army Army)
    (if (== (.unit _array_element) Unit)
      (|SetBy-RefVar (.quantity (Utilities|Array|Get(acopy) (.army Army) _array_index)) (Math|Integer|Max(Integer) (- (.quantity _array_element) Quantity)))
      (return))))

(fn IsDefeated
  (params (Army :type ST%20Army%20Structure%20%28by%20ref%29))
  (for _array_element (.army Army)
    (if (!= (.quantity _array_element) 0)
      (return false)))
  (return true))

(fn GetArmyDataforUnit
  (params (Army :type ST%20Army%20Structure%20%28by%20ref%29) (Unit :type BP%20Unit%20Base%20Class%20Reference))
  (for _array_element (.army Army)
    (if (== (.Unit (Utilities|Struct|BreakST_ArmyData _array_element)) Unit)
      (return _array_element)))
  (return (Utilities|Struct|MakeST_ArmyData 0 -1)))

(fn HasAnyAvailableUnitRemaining
  (params (Army :type ST%20Army%20Structure) (Unit :type BP%20Unit%20Base%20Class%20Reference))
  (return (> (CallFunction|GetRemainingUnitCount Army Unit) 0)))

(fn GetRemainingUnitCount
  (params (Army :type ST%20Army%20Structure) (Unit :type BP%20Unit%20Base%20Class%20Reference))
  (bind _data (CallFunction|GetArmyDataforUnit Army Unit))
  (if (Utilities|IsValidClass (.unit _data))
    (for _array_element (.engagedarmy Army)
      (if (== (.Unit (Utilities|Struct|BreakST_ArmyData _array_element)) Unit)
        (return (- (.quantity _data) (.Quantity (Utilities|Struct|BreakST_ArmyData _array_element))))))
    (return (.quantity _data))
    (else
      (return 0))))

(fn AddUnitinEngagedList
  (params (Army :type ST%20Army%20Structure%20%28by%20ref%29) (Unit :type BP%20Unit%20Base%20Class%20Reference) (QuantityToEngage :type Integer))
  (for (_array_element _array_index) (.engagedarmy Army)
    (if (== (.unit _array_element) Unit)
      (|SetBy-RefVar (.quantity (Utilities|Array|Get(acopy) (.engagedarmy Army) _array_index)) (+ (.quantity _array_element) QuantityToEngage))
      (return)))
  (Utilities|Array|Add (.engagedarmy Army) (Utilities|Struct|MakeST_ArmyData Unit QuantityToEngage)))

(fn RemoveUnitinEngagedList
  (params (Army :type ST%20Army%20Structure%20%28by%20ref%29) (Unit :type BP%20Unit%20Base%20Class%20Reference) (QuantityToEngage :type Integer))
  (for (_array_element _array_index) (.engagedarmy Army)
    (if (== (.unit _array_element) Unit)
      (|SetBy-RefVar (.quantity (Utilities|Array|Get(acopy) (.engagedarmy Army) _array_index)) (Math|Integer|Max(Integer) (- (.quantity _array_element) QuantityToEngage)))
      (return))))

(fn IsUnitStrongAgainst
  (params (UnitRef :type ST%20Unit%20Data%20Structure) (OppositeUnit :type ST%20Unit%20Data%20Structure))
  (bind _newparam (CallFunction|IsModifierStrongAgainst UnitRef OppositeUnit))
  (switch Utilities|FlowControl|Switch|SwitchonE_EncounterResults (CallFunction|IsWeaponStrongAgainst UnitRef OppositeUnit)
    (:NewEnumerator0
      (switch Utilities|FlowControl|Switch|SwitchonE_EncounterResults _newparam
        (:NewEnumerator0
          _)
        (:NewEnumerator1
          _)
        (:NewEnumerator2
          _)
        (:NewEnumerator3
          (return "NewEnumerator1"))
        (:NewEnumerator4
          (return "NewEnumerator2"))))
    (:NewEnumerator1
      (switch Utilities|FlowControl|Switch|SwitchonE_EncounterResults _newparam
        (:NewEnumerator0
          _)
        (:NewEnumerator1
          _)
        (:NewEnumerator2
          (return "NewEnumerator1"))
        (:NewEnumerator3
          (return "NewEnumerator2"))
        (:NewEnumerator4
          (return "NewEnumerator3"))))
    (:NewEnumerator2
      (switch Utilities|FlowControl|Switch|SwitchonE_EncounterResults _newparam
        (:NewEnumerator0
          _)
        (:NewEnumerator1
          (return "NewEnumerator1"))
        (:NewEnumerator2
          (return "NewEnumerator2"))
        (:NewEnumerator3
          (return "NewEnumerator3"))
        (:NewEnumerator4
          (return "NewEnumerator4"))))
    (:NewEnumerator3
      (switch Utilities|FlowControl|Switch|SwitchonE_EncounterResults _newparam
        (:NewEnumerator0
          (return "NewEnumerator1"))
        (:NewEnumerator1
          (return "NewEnumerator2"))
        (:NewEnumerator2
          (return "NewEnumerator3"))
        (:NewEnumerator3
          _)
        (:NewEnumerator4
          _))
      (return "NewEnumerator4"))
    (:NewEnumerator4
      (switch Utilities|FlowControl|Switch|SwitchonE_EncounterResults _newparam
        (:NewEnumerator0
          (return "NewEnumerator2"))
        (:NewEnumerator1
          (return "NewEnumerator3"))
        (:NewEnumerator2
          _)
        (:NewEnumerator3
          _)
        (:NewEnumerator4
          _))
      (return "NewEnumerator4")))
  (return "NewEnumerator0"))

(fn IsWeaponStrongAgainst
  (params (Reference :type ST%20Unit%20Data%20Structure) (Opposite :type ST%20Unit%20Data%20Structure))
  (switch Utilities|FlowControl|Switch|SwitchonE_UnitType (.unittype Reference)
    (:NewEnumerator0
      (switch Utilities|FlowControl|Switch|SwitchonE_UnitType (.unittype Opposite)
        (:NewEnumerator0
          _)
        (:NewEnumerator2
          (return "NewEnumerator1"))
        (:NewEnumerator3
          (return "NewEnumerator3"))
        (:NewEnumerator1
          _)))
    (:NewEnumerator2
      (switch Utilities|FlowControl|Switch|SwitchonE_UnitType (.unittype Opposite)
        (:NewEnumerator0
          (return "NewEnumerator3"))
        (:NewEnumerator2
          _)
        (:NewEnumerator3
          (return "NewEnumerator1"))
        (:NewEnumerator1
          _)))
    (:NewEnumerator3
      (switch Utilities|FlowControl|Switch|SwitchonE_UnitType (.unittype Opposite)
        (:NewEnumerator0
          (return "NewEnumerator1"))
        (:NewEnumerator2
          (return "NewEnumerator3"))
        (:NewEnumerator3
          _)
        (:NewEnumerator1
          _)))
    (:NewEnumerator1
      (if (Utilities|Enum|Equal(Enum) (.unitmodifier Opposite) "NewEnumerator2")
        (return "NewEnumerator3")
        (else
          _))))
  (return "NewEnumerator2"))

(fn IsModifierStrongAgainst
  (params (Reference :type ST%20Unit%20Data%20Structure) (Opposite :type ST%20Unit%20Data%20Structure))
  (switch Utilities|FlowControl|Switch|SwitchonE_UnitModifier (.unitmodifier Reference)
    (:NewEnumerator0
      (switch Utilities|FlowControl|Switch|SwitchonE_UnitModifier (.unitmodifier Opposite) :!label _label
        (:NewEnumerator0
          _)
        (:NewEnumerator1
          _)
        (:NewEnumerator2
          (return "NewEnumerator1"))
        (:NewEnumerator3
          _)))
    (:NewEnumerator1
      (goto _label))
    (:NewEnumerator2
      (switch Utilities|FlowControl|Switch|SwitchonE_UnitModifier (.unitmodifier Opposite)
        (:NewEnumerator0
          (return "NewEnumerator3"))
        (:NewEnumerator1
          (return "NewEnumerator3"))
        (:NewEnumerator2
          _)
        (:NewEnumerator3
          (return "NewEnumerator3"))))
    (:NewEnumerator3
      (goto _label)))
  (return "NewEnumerator2"))

(fn IsBetterEncounter
  (params (A :type E_EncounterResults%20Enum :default "NewEnumerator0") (B :type E_EncounterResults%20Enum :default "NewEnumerator0"))
  (switch Utilities|FlowControl|Switch|SwitchonE_EncounterResults A
    (:NewEnumerator0
      (return false))
    (:NewEnumerator1
      (switch Utilities|FlowControl|Switch|SwitchonE_EncounterResults B
        (:NewEnumerator0
          _)
        (:NewEnumerator1
          (return false))
        (:NewEnumerator2
          (return false))
        (:NewEnumerator3
          (return false))
        (:NewEnumerator4
          (return false))))
    (:NewEnumerator2
      (switch Utilities|FlowControl|Switch|SwitchonE_EncounterResults B
        (:NewEnumerator0
          _)
        (:NewEnumerator1
          _)
        (:NewEnumerator2
          (return false))
        (:NewEnumerator3
          (return false))
        (:NewEnumerator4
          (return false))))
    (:NewEnumerator3
      (switch Utilities|FlowControl|Switch|SwitchonE_EncounterResults B
        (:NewEnumerator0
          _)
        (:NewEnumerator1
          _)
        (:NewEnumerator2
          _)
        (:NewEnumerator3
          (return false))
        (:NewEnumerator4
          (return false))))
    (:NewEnumerator4
      (return true)))
  (return true))